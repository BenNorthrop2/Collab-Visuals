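; BP_CrossProdTest is a test Blueprint that visualizes a vector cross product with cube components.
; Each Tick it normalizes the world locations of Cube2 and Cube1, crosses them, and sets the relative rotation of Cube so its Z axis follows the result.
; The vectors are measured from the world origin, and an unconnected node chain multiplying a second cross product involving Cube3 is left unused.
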(event EventTick
  (params (DeltaSeconds :type Float%20%28single-precision%29))
  (Transformation|SetRelativeRotation (Variables|Default|GetCube) (Math|Rotator|MakeRotfromZ (Math|Vector|CrossProduct (Math|Vector|Normalize (Transformation|GetWorldLocation (Variables|Default|GetCube2))) (Math|Vector|Normalize (Transformation|GetWorldLocation (Variables|Default|GetCube1))))) false false))

(fn ConstructionScript)